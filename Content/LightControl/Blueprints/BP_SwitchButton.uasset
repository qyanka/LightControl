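; BP_SwitchButton is a pressure button actor that fires its OnPressed dispatcher when BP_ThirdPersonCharacter overlaps it.
; The ButtonMove timeline feeds a macro that lerps Z toward half the actor scale cached at BeginPlay, squashing the Cube to fake a press.
; Ending the overlap reverses the timeline from its end to raise the button again.
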(event `self.ReceiveBeginPlay`
  ; Сохранение начального скейла кнопки
  (set `self.InitialScale` (`self.GetActorRelativeScale3D`)))

(event `self.ReceiveActorBeginOverlap`
  (params (OtherActor :type "Actor Object Reference"))
  ; Реакция кнопки на оверлап с персонажем
  (cast `/Game/ThirdPerson/Blueprints/BP_ThirdPersonCharacter` OtherActor)
  (`self.OnPressed`)
  ; Вычисление скейла для имитации нажатия кнопки с помощю таймлайна
  (bind (_direction _newtrack_0) (`Timeline|ButtonMove` :!label _label)
    (:`Update`
      (bind (_cube _initialscale_x _initialscale_y _returnvalue) (`self.NewMacro` _newtrack_0))
      (`SceneComponent.SetRelativeScale3D` _cube (`KismetMathLibrary.MakeVector` _initialscale_x _initialscale_y _returnvalue)))))

(event `self.ReceiveActorEndOverlap`
  (params (OtherActor :type "Actor Object Reference"))
  ; Реакция кнопки на оверлап с персонажем
  (cast `/Game/ThirdPerson/Blueprints/BP_ThirdPersonCharacter` OtherActor)
  (goto _label :!via `ReverseFromEnd`))

(fn `UserConstructionScript`)