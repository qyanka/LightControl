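; BP_Lightbulb is an interactable light source that can be switched on and off.
; Interact calls the bulb's own Toggle event only when the Interactor implements BPI_Switchable.
; Toggle inverts the visibility of the PointLight component without propagating to its children.
; GetInteractionText supplies a fixed key prompt for toggling.
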(event `/Game/LightControl/Blueprints/Interfaces/BPI_Interactable.Interact`
  (params (Interactor :type "Actor Object Reference"))
  ; Реализация взаимодействия с Interactable сущностью
  (if (`KismetSystemLibrary.DoesImplementInterface` Interactor "/Game/LightControl/Blueprints/Interfaces/BPI_Switchable.BPI_Switchable_C")
    (`self.Toggle`)))

(event `/Game/LightControl/Blueprints/Interfaces/BPI_Switchable.Toggle`
  ; Изменение Visibility у источника света
  (`SceneComponent.SetVisibility` (`self.PointLight`) (not (`SceneComponent.IsVisible` (`self.PointLight`))) false))

(fn `GetInteractionText`
  (returns (Text :type Text))
  (return "Press E to toggle"))

(fn `UserConstructionScript`)